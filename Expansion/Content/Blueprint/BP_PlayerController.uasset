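; Player-controlled physics mesh that grows by eating BP_Food.
; WASD keys set forward and right values, which Tick feeds as yaw and pitch angles into a unit-length acceleration force, so it points roughly along +X even without input.
; Food entering FoodTrigger is told to move towards the mesh's location.
; Mesh overlap adds the food's increase to FoodAmount and sets that as world scale.
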(event OnComponentBeginOverlap(FoodTrigger)
  (params (OverlappedComponent :type Primitive%20Component%20Object%20Reference) (OtherActor :type Actor%20Object%20Reference) (OtherComp :type Primitive%20Component%20Object%20Reference) (OtherBodyIndex :type Integer) (bFromSweep :type Boolean) (SweepResult :type Hit%20Result%20Structure%20%28by%20ref%29))
  (bind _asbp_food (Utilities|Casting|CastToBP_Food OtherActor))
  (Default|MoveTowards _asbp_food (Transformation|GetWorldLocation (Variables|Character|GetMesh))))

(event OnComponentBeginOverlap(Mesh)
  (params (OverlappedComponent :type Primitive%20Component%20Object%20Reference) (OtherActor :type Actor%20Object%20Reference) (OtherComp :type Primitive%20Component%20Object%20Reference) (OtherBodyIndex :type Integer) (bFromSweep :type Boolean) (SweepResult :type Hit%20Result%20Structure%20%28by%20ref%29))
  (bind _asbp_food (Utilities|Casting|CastToBP_Food OtherActor))
  (bind _output_get (Variables|Default|SetFoodAmount (+ (Variables|/Game/Blueprint/BP_Food.BP_Food_C|GetFoodIncrease _asbp_food) (Variables|Default|GetFoodAmount))))
  (Transformation|SetWorldScale3D (Variables|Character|GetMesh) (Math|Conversions|ToVector(Float) _output_get)))

(event EventBeginPlay)

(event Collision|EventActorBeginOverlap
  (params (OtherActor :type Actor%20Object%20Reference)))

(event EventTick
  (params (DeltaSeconds :type Float%20%28single-precision%29))
  (Physics|AddForce (Variables|Character|GetMesh) (Class|KismetMathLibrary|CreateVectorfromYawPitch (Math|Conversions|ToFloat(Integer) (Variables|Default|GetForwardDir)) (Math|Conversions|ToFloat(Integer) (Variables|Default|GetRightDir)) 1.0) "None" true))

(event Input|KeyboardEvents|W
  (params (Key :type Key%20Structure :default "None"))
  (:Pressed
    (Variables|Default|SetForwardDir 1))
  (:Released
    (Variables|Default|SetForwardDir 0)))

(event Input|KeyboardEvents|S
  (params (Key :type Key%20Structure :default "None"))
  (:Pressed
    (Variables|Default|SetForwardDir -1))
  (:Released
    (Variables|Default|SetForwardDir 0)))

(event Input|KeyboardEvents|A
  (params (Key :type Key%20Structure :default "None"))
  (:Pressed
    (Variables|Default|SetRightDir 1))
  (:Released
    (Variables|Default|SetRightDir 0)))

(event Input|KeyboardEvents|D
  (params (Key :type Key%20Structure :default "None"))
  (:Pressed
    (Variables|Default|SetRightDir -1))
  (:Released
    (Variables|Default|SetRightDir 0)))

(fn ConstructionScript)