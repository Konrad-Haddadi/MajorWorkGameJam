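; BP_Food is a food actor whose mesh can be given a target position to move towards.
; MoveTowards stores the target and sets IsMoving, which nothing in this graph clears.
; While moving, Tick sets FoodMesh's world location to the target offset times DeltaSeconds, without adding the current location, so the mesh does not converge on the target.
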(event EventBeginPlay)

(event Collision|EventActorBeginOverlap
  (params (OtherActor :type Actor%20Object%20Reference)))

(event EventTick
  (params (DeltaSeconds :type Float%20%28single-precision%29))
  (if (Variables|Default|GetisMoving)
    (Transformation|SetWorldLocation (Variables|Default|GetFoodMesh) (* (- (Variables|Default|GetTargetPos) (Transformation|GetWorldLocation (Variables|Default|GetFoodMesh))) DeltaSeconds) false false)))

(fn ConstructionScript)

(fn MoveTowards
  (params (TargetPosition :type Vector))
  (Variables|Default|SetTargetPos TargetPosition)
  (Variables|Default|SetisMoving true))