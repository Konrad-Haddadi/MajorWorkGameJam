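; Player character that grows by absorbing BP_Food actors.
; Food entering FoodTrigger is told to move toward the BodyTemp mesh's location, sampled once when the overlap begins.
; When BodyTemp hits food, its BoostAmount is added to PlayerLevel, which becomes the mesh's uniform world scale.
; The construction script assigns the StaticMesh variable to BodyTemp, and this Blueprint leaves removal of eaten food to other code.
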(event OnComponentBeginOverlap(FoodTrigger)
  (params (OverlappedComponent :type Primitive%20Component%20Object%20Reference) (OtherActor :type Actor%20Object%20Reference) (OtherComp :type Primitive%20Component%20Object%20Reference) (OtherBodyIndex :type Integer) (bFromSweep :type Boolean) (SweepResult :type Hit%20Result%20Structure%20%28by%20ref%29))
  (bind _asbp_food (Utilities|Casting|CastToBP_Food OtherActor))
  (Default|MoveTowards _asbp_food (Transformation|GetWorldLocation (Variables|Default|GetBodyTemp))))

(event OnComponentHit(BodyTemp)
  (params (HitComponent :type Primitive%20Component%20Object%20Reference) (OtherActor :type Actor%20Object%20Reference) (OtherComp :type Primitive%20Component%20Object%20Reference) (NormalImpulse :type Vector :default "0, 0, 0") (Hit :type Hit%20Result%20Structure%20%28by%20ref%29))
  (bind _asbp_food (Utilities|Casting|CastToBP_Food OtherActor))
  (bind _output_get (Variables|Default|SetPlayerLevel (+ (Variables|Default|GetPlayerLevel) (Variables|/Game/ExpandingContent/Blueprint/BP_Food.BP_Food_C|GetBoostAmount _asbp_food))))
  (Transformation|SetWorldScale3D (Variables|Default|GetBodyTemp) (Math|Conversions|ToVector(Float) _output_get)))

(event EventBeginPlay)

(event Collision|EventActorBeginOverlap
  (params (OtherActor :type Actor%20Object%20Reference)))

(event EventTick
  (params (DeltaSeconds :type Float%20%28single-precision%29)))

(fn ConstructionScript
  (Components|StaticMesh|SetStaticMesh (Variables|Default|GetBodyTemp) (Variables|Default|GetStaticMesh)))